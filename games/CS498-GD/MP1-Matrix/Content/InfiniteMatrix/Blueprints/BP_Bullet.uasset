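; BP_Bullet is a projectile owned by BP_Player that destroys enemies and awards score.
; Tick sweeps it along local X at the player's forward speed plus its own movement speed, scaled down for rockets.
; Hitting a BP_Enemy destroys both, raises score relative to the current total and plays a death sound at the player.
; BP_Tunnel hits are left to the tunnel's logic, while other hits destroy the bullet.
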(event OnComponentHit(Bullet)
  (params (HitComponent :type Primitive%20Component%20Object%20Reference) (OtherActor :type Actor%20Object%20Reference) (OtherComp :type Primitive%20Component%20Object%20Reference) (NormalImpulse :type Vector :default "0, 0, 0") (Hit :type Hit%20Result%20Structure%20%28by%20ref%29))
  (bind _asbp_enemy (Utilities|Casting|CastToBP_Enemy OtherActor)
    (:then
      (Actor|DestroyActor _asbp_enemy)
      (bind _asbp_player (Utilities|Casting|CastToBP_Player (Components|GetOwner)))
      (Default|ChangeScore _asbp_player (+ (/ (Variables|/Game/InfiniteMatrix/Blueprints/BP_Player.BP_Player_C|GetGameScore _asbp_player) 50) 1) true)
      (Utilities|FlowControl|Sequence
        (:then_0
          (Audio|PlaySoundatLocation "/Game/InfiniteMatrix/Audio/death.death" (Transformation|GetActorLocation _asbp_player) "0, 0, 0" 0.5 1.0 0.0 0 0 0))
        (:then_1
          (Actor|DestroyActor :!label _label))))
    (:CastFailed
      (Utilities|Casting|CastToBP_Tunnel OtherActor ; If it is a tunnel, let the tunnel logic handle it, else kill it
        (:CastFailed
          (goto _label))))))

(event EventBeginPlay)

(event Collision|EventActorBeginOverlap
  (params (OtherActor :type Actor%20Object%20Reference)))

(event EventTick
  (params (DeltaSeconds :type Float%20%28single-precision%29))
  (bind _asbp_player (Utilities|Casting|CastToBP_Player (Components|GetOwner)))
  (Transformation|AddLocalOffset (Variables|Default|GetBullet) (Math|Vector|MakeVector (select (Variables|Default|GetIsRocket) (* (+ (Variables|/Game/InfiniteMatrix/Blueprints/BP_Player.BP_Player_C|GetForwardSpeed _asbp_player) (Variables|Default|GetMovementSpeed)) 0.6 DeltaSeconds) (* DeltaSeconds (+ (Variables|/Game/InfiniteMatrix/Blueprints/BP_Player.BP_Player_C|GetForwardSpeed _asbp_player) (Variables|Default|GetMovementSpeed)))) 0.0 0.0) true false))

(fn ConstructionScript)