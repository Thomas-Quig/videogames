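; BP_Enemy is a hazard actor that damages the player on contact.
; On BeginPlay it randomly picks a clockwise or counter-clockwise spin, and Tick yaws its Cube at that rate, scaled by delta time.
; When the Cube hits a BP_Player, it removes one health through ChangeHealth, plays a damage sound at the player's location and destroys itself.
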(event OnComponentHit(Cube)
  (params (HitComponent :type Primitive%20Component%20Object%20Reference) (OtherActor :type Actor%20Object%20Reference) (OtherComp :type Primitive%20Component%20Object%20Reference) (NormalImpulse :type Vector :default "0, 0, 0") (Hit :type Hit%20Result%20Structure%20%28by%20ref%29))
  (bind _asbp_player (Utilities|Casting|CastToBP_Player OtherActor))
  (Default|ChangeHealth _asbp_player -1)
  (Audio|PlaySoundatLocation "/Game/InfiniteMatrix/Audio/damage_Cue.damage_Cue" (Transformation|GetActorLocation _asbp_player) "0, 0, 0" 1.0 1.0 0.0 0 0 0)
  (Actor|DestroyActor))

(event EventBeginPlay
  (if (Math|Random|RandomBool)
    (Variables|Default|SetRotationSpeed 9e+01)
    (else
      (Variables|Default|SetRotationSpeed -9e+01))))

(event EventTick
  (params (DeltaSeconds :type Float%20%28single-precision%29))
  (Transformation|AddLocalRotation (Variables|Default|GetCube) (Math|Rotator|MakeRotator 0.0 0.0 (* DeltaSeconds (Variables|Default|GetRotationSpeed))) false false))

(fn ConstructionScript)